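; AC_Mine is a falling mine hazard that damages the player's paper ship on contact.
; On BeginPlay it starts a looping timer, with an interval derived from GetFramePace, that steps the actor down along Z at a fixed increment.
; When its Box overlaps an actor tagged Player that casts to BP_PaperShip, it calls Damage on the ship and destroys itself.
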(event OnComponentBeginOverlap(Box)
  (params (OverlappedComponent :type Primitive%20Component%20Object%20Reference) (OtherActor :type Actor%20Object%20Reference) (OtherComp :type Primitive%20Component%20Object%20Reference) (OtherBodyIndex :type Integer) (bFromSweep :type Boolean) (SweepResult :type Hit%20Result%20Structure%20%28by%20ref%29))
  ;[1 1 1] 当たり判定の処理
  (if (Actor|ActorHasTag OtherActor "Player")
    (bind _asbp_paper_ship (Utilities|Casting|CastToBP_PaperShip OtherActor))
    (Default|Damage _asbp_paper_ship)
    (Actor|DestroyActor)))

(event Custom|Fall
  (bind _returnvalue (Transformation|GetActorLocation))
  ;[1 1 1] 落ちるイベントをタイマーで呼び出す
  (Transformation|SetActorLocation (Math|Vector|MakeVector (.x _returnvalue) (.y _returnvalue) (- (.z _returnvalue) 2.0)) false false))

(event EventBeginPlay
  (Utilities|Time|SetTimerbyEvent (delegate Custom|Fall) (/ 1.0 (Math|Conversions|ToFloat(Integer) (Class|GameUserSettings|GetFramePace))) true))

(fn ConstructionScript)