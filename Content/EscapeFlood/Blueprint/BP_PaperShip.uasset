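; Touch-controlled paper ship for EscapeFlood that can sink and resurface, with an HP widget shown on screen.
; Touch input sets its X/Y position, with X measured from the viewport center.
; A Tick state machine holds height in Stand, lowers the ship for a frame countdown in Fall, then raises it by the same step count in Float.
; External events trigger falling, floating after leaving a rock, and the widget's damage message.
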(event Custom|UpdatePosition
  (params (StartPosition :type Vector%202D%20Structure))
  (bind _position (Variables|Default|GetPosition))
  (bind _returnvalue (- StartPosition _position))
  ;[1 1 1] タッチへの追従
  (switch Utilities|FlowControl|Switch|SwitchonPlayerState (Variables|Default|GetEPlayerState)
    (:NewEnumerator0
      (Transformation|SetWorldLocation (Variables|Collision|GetCapsuleComponent) (Math|Vector|MakeVector (.x _returnvalue) (.y _returnvalue) (Variables|Default|GetInitZ)) false false))))

(event Custom|FallPlayer
  (bind _position (Variables|Default|GetPosition))
  (bind _capsulecomponent (Variables|Collision|GetCapsuleComponent))
  (bind _returnvalue (Transformation|GetWorldLocation _capsulecomponent))
  ;[1 1 1] 落ちる
  (Transformation|SetWorldLocation (Variables|Collision|GetCapsuleComponent) (Math|Vector|MakeVector (.x _position) (.y _position) (- (.z _returnvalue) (/ (Variables|Default|GetFallSpeed) 6e+01))) false false)
  (bind _result (Math|Integer|IncrementInt (Variables|Default|GetCount))
    (:%20%20
      (Development|PrintString (Utilities|String|ToString(Float) (.z _returnvalue))))))

(event Custom|Float
  (bind _position (Variables|Default|GetPosition))
  ;[1 1 1] 岩から離れた時に浮上する
  (Transformation|SetWorldLocation (Variables|Collision|GetCapsuleComponent) (Math|Vector|MakeVector (.x _position) (.y _position) (- (.z (Transformation|GetActorLocation)) (* -1 (/ (Variables|Default|GetFallSpeed) 6e+01)))) false false))

(event EventBeginPlay
  (UserInterface|Viewport|AddtoViewport (UserInterface|GetWidget (Variables|Default|GetHP)) 0))

(event EventFall
  (Variables|Default|SetEPlayerState "NewEnumerator1"))

(event EventTick
  (params (DeltaSeconds :type Float%20%28single-precision%29))
  (bind _position (Variables|Default|GetPosition))
  (switch Utilities|FlowControl|Switch|SwitchonPlayerState (Variables|Default|GetEPlayerState)
    (:NewEnumerator0
      (Transformation|SetWorldLocation (Variables|Collision|GetCapsuleComponent) (Math|Vector|MakeVector (.x _position) (.y _position) (Variables|Default|GetInitZ)) false false))
    (:NewEnumerator1
      (CallFunction|FallPlayer)
      (Math|Integer|IncrementInt (Variables|Default|GetFallTimes)
        (:%20%20
          (if (< (Variables|Default|GetFloatCount) 0)
            (Variables|Default|SetEPlayerState "NewEnumerator2")
            (Variables|Default|SetFloatCount 20)
            (Variables|Default|SetCount 0)
            (else
              (Math|Integer|DecrementInt (Variables|Default|GetFloatCount)))))))
    (:NewEnumerator2
      (switch int (Variables|Default|GetFallTimes)
        (:Default
          (CallFunction|Float)
          (Math|Integer|DecrementInt (Variables|Default|GetFallTimes)))
        (:0
          (Variables|Default|SetEPlayerState "NewEnumerator0"))))))

(event EventDamage
  (Class|Damage|Damage(Message) (UserInterface|GetWidget (Variables|Default|GetHP))))

(event EventNoHitRock
  (Variables|Default|SetEPlayerState "NewEnumerator2"))

(event Input|TouchEvents|InputTouch
  (params (Location :type Vector) (FingerIndex :type ETouchIndex%20Enum))
  (bind _returnvalue (Viewport|GetViewportSize))
  (bind _returnvalue_2 (/ (.x _returnvalue) 2.0))
  (bind _returnvalue_3 (- (.x Location) _returnvalue_2))
  ;[1 1 1] タッチへの追従
  (:Pressed
    (Variables|Default|SetIsTouched true)
    (Variables|Default|SetPosition (Math|Vector2D|MakeVector2D _returnvalue_3 (.y Location)) :!label _label))
  (:Released
    (Variables|Default|SetIsTouched false)
    (goto _label))
  (:Moved
    (CallFunction|UpdatePosition (Math|Vector2D|MakeVector2D _returnvalue_3 (.y Location)))
    (goto _label)))

(fn ConstructionScript)