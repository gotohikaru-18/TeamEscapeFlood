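; AC_GimmickSpawner is an obstacle spawner that periodically places random mines or rocks above the player in EscapeFlood.
; BeginPlay fills the class list with AC_Mine and AC_Rock and starts a looping Spawn timer, which MainGameStart can also start.
; Spawn picks a random class and places it at a fixed Y, above the player, with random X around the player spanning the viewport's pixel width as world units.
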(event Custom|MainGameStart
  (Utilities|Time|SetTimerbyEvent (delegate Custom|Spawn) (Variables|Default|GetSpawnTIme) true))

(event Custom|Spawn
  (bind _returnvalue (Game|Player|GetPlayerPawn 0))
  (bind _returnvalue_2 (Viewport|GetViewportSize))
  (bind _returnvalue_3 (Transformation|GetActorLocation _returnvalue))
  (Game|SpawnActorfromClass (.OutItem (Utilities|Array|Random (Variables|Default|GetGimmickClasses))) (Math|Transform|MakeTransform (Math|Vector|MakeVector (+ (Math|Random|RandomFloatinRange (/ (.x _returnvalue_2) -2.0) (/ (.x _returnvalue_2) 2.0)) (.x _returnvalue_3)) 5e+01 (+ (.z _returnvalue_3) 3e+02)) "0, 0, 0" "1,1,1") "Undefined" 0 0))

(event EventBeginPlay
  (bind _gimmickclasses (Variables|Default|GetGimmickClasses))
  (Utilities|Array|Add _gimmickclasses "/Game/EscapeFlood/Blueprint/AC_Mine.AC_Mine_C")
  (Utilities|Array|Add _gimmickclasses "/Game/EscapeFlood/Blueprint/AC_Rock.AC_Rock_C")
  (Utilities|Time|SetTimerbyEvent (delegate Custom|Spawn) (Variables|Default|GetSpawnTIme) true))

(fn ConstructionScript)